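; BP_Ice is an ice actor that randomizes its own rotation and size when play begins.
; BeginPlay keeps the location and multiplies each rotation and scale axis by an independent random factor, with a narrower range for vertical scale.
; Because rotation is multiplied rather than offset, axes at zero stay unrotated.
; Overlap, Tick and the construction script do nothing.
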(event `self.ReceiveBeginPlay`
  (`self.K2_SetActorTransform` (`KismetMathLibrary.MakeTransform` (.location (`self.GetTransform`)) (`KismetMathLibrary.MakeRotator` (* (.roll (.rotation (`self.GetTransform`))) (`KismetMathLibrary.RandomFloatInRange` 1.0 10.0)) (* (.pitch (.rotation (`self.GetTransform`))) (`KismetMathLibrary.RandomFloatInRange` 1.0 10.0)) (* (.yaw (.rotation (`self.GetTransform`))) (`KismetMathLibrary.RandomFloatInRange` 1.0 10.0))) (`KismetMathLibrary.MakeVector` (* (.x (.scale (`self.GetTransform`))) (`KismetMathLibrary.RandomFloatInRange` 1.0 10.0)) (* (.y (.scale (`self.GetTransform`))) (`KismetMathLibrary.RandomFloatInRange` 1.0 10.0)) (* (.z (.scale (`self.GetTransform`))) (`KismetMathLibrary.RandomFloatInRange` 1.0 5.0))))))

(event `self.ReceiveTick`
  (params (DeltaSeconds :type "Float (single-precision)")))

(fn `UserConstructionScript`)